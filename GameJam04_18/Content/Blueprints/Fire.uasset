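; Fire hazard actor that kills the player's Sedan on contact and can be put out with water.
; On BeginPlay it attaches a scaled fire particle emitter to its static mesh.
; Collision overlaps with an actor whose first tag is Player call Death on the player pawn, cast to Sedan.
; Each WaterCollision event decrements FireHP and destroys the actor once it is depleted.
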(event OnComponentBeginOverlap(Collision)
  (params (OverlappedComponent :type Primitive%20Component%20Object%20Reference) (OtherActor :type Actor%20Object%20Reference) (OtherComp :type Primitive%20Component%20Object%20Reference) (OtherBodyIndex :type Integer) (bFromSweep :type Boolean) (SweepResult :type Hit%20Result%20Structure%20%28by%20ref%29))
  (bind _tags (Variables|/Script/Engine.Actor|GetTags OtherActor))
  (if (Utilities|Array|IsValidIndex _tags)
    (switch name (Utilities|Array|Get(acopy) _tags)
      (:Player
        (bind _assedan (Utilities|Casting|CastToSedan (Game|Player|GetPlayerPawn 0)))
        (Default|Death _assedan)))))

(event Custom|WaterCollision
  (Variables|Default|SetFireHP (- (Variables|Default|GetFireHP) 1))
  (if (<= (Variables|Default|GetFireHP) 0)
    (Actor|DestroyActor)))

(event EventBeginPlay
  (Effects|SpawnEmitterAttached "/Game/P_Forge_IB_Fire.P_Forge_IB_Fire" (Variables|Debug|GetStaticMeshComponent) "None" "0, 0, 0" "0, 0, 0" "3.000000,3.000000,3.000000" "KeepRelativeOffset" false))

(event Collision|EventActorBeginOverlap
  (params (OtherActor :type Actor%20Object%20Reference)))

(event EventTick
  (params (DeltaSeconds :type Float%20%28single-precision%29)))

(fn ConstructionScript)